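; Parkour movement component that gives a character wall running, wall jumping and camera tilt.
; After initialization, a looping timer line-traces right, then left, and on valid airborne hits launches the character along the wall while easing gravity toward a target.
; Ending a run restores gravity and briefly suppresses re-attachment; jumping launches off the wall normal, and landing clears suppression.
; Tick interpolates control-rotation roll according to the wall side.
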(event `self.ReceiveTick`
  (params (DeltaSeconds :type "Float (single-precision)"))
  (`self.CameraTick`))

(event `Initialize`
  (params (Character_REF :type "Character Object Reference"))
  (bind _output_get (set `self.Character REF` Character_REF))
  (bind _output_get_2 (set `self.Character Movement` (`Character.CharacterMovement` _output_get)))
  (set `self.Default Gravity Scale` (`CharacterMovementComponent.GravityScale` _output_get_2))
  (`KismetSystemLibrary.K2_SetTimerDelegate` (delegate `WallRunUpdateEvent`) 0.02 true))

(event `LandEvent`
  (`self.WallRunEnd` 0.0)
  (set `self.WallRunSupressed?` false))

(event `JumpEvent`
  (`self.JumpFromWall`))

(event `ResetWallRunSupressed`
  (`KismetSystemLibrary.K2_ClearTimer` null "ResetWallRunSupressed")
  (set `self.WallRunSupressed?` false))

(event `WallRunUpdateEvent`
  (if (not (`self.WallRunSupressed?`))
    (`self.WallRunUpdate `)))

(fn `CameraTick`
  (if (`self.WallRunnig?Left`)
    (`self.CameraTilty` 15.0)
    (elif (`self.WallRunnig?Right`)
      (`self.CameraTilty` -15.0)
      (else
        (`self.CameraTilty` 0.0)))))

(fn `CameraTilty`
  (params (`Target X (Roll)` :type "Float (double-precision)"))
  (bind _returnvalue (`Controller.GetControlRotation` (`Pawn.GetController` (`self.Character REF`))))
  (`Controller.SetControlRotation` (`Pawn.GetController` (`self.Character REF`)) (`KismetMathLibrary.RInterpTo` _returnvalue (`KismetMathLibrary.MakeRotator` `Target X (Roll)` (.pitch _returnvalue) (.yaw _returnvalue)) (`GameplayStatics.GetWorldDeltaSeconds`) 10.0)))

(fn `JumpFromWall`
  (bind (_outvec_x _outvec_y) (`KismetMathLibrary.BreakVector` (`self.OutVec`)))
  (bind _jumppower (`self.JumpPower`))
  (if (`self.WallRunnig?`)
    (`self.WallRunEnd` 0.35)
    (`Character.LaunchCharacter` (`self.Character REF`) (`KismetMathLibrary.MakeVector` (* _jumppower _outvec_x) (* _jumppower _outvec_y) (`self.WallJump`)) false true)))

(fn `SupressedWallRun`
  (params (Delay :type "Float (double-precision)"))
  (set `self.WallRunSupressed?` true)
  (`KismetSystemLibrary.K2_SetTimer` null "ResetWallRunSupressed" Delay))

(fn `WallRunEnd`
  (params (ResetTime :type "Float (double-precision)"))
  (if (`self.WallRunnig?`)
    (set `self.WallRunnig?` false)
    (set `self.WallRunnig?Right` false)
    (set `self.WallRunnig?Left` false)
    (set `CharacterMovementComponent.GravityScale` (`self.Default Gravity Scale`) (`self.Character Movement`))
    (`self.SupressedWallRun` ResetTime)))

(fn `WallRunMovement`
  (params (Start :type "Vector Structure") (End :type "Vector Structure") (Direction :type "Float (double-precision)"))
  (returns (`OnWall?` :type Boolean))
  (bind _outhit (`KismetSystemLibrary.LineTraceSingle` Start End "TraceTypeQuery1"))
  (if (`GameplayStatics.BreakHitResult` _outhit)
    (bind (_returnvalue _invec2) (`self.ValidWallRunActor` (`.Normal` (`GameplayStatics.BreakHitResult` _outhit))))
    (if (and _returnvalue (`NavMovementComponent.IsFalling` (`self.Character Movement`)))
      (set `self.OutVec` _invec2)
      (`Character.LaunchCharacter` (`self.Character REF`) (`self.PlayerToWallvector`) false false)
      (`Character.LaunchCharacter` (`self.Character REF`) (* (`KismetMathLibrary.Cross_VectorVector` (`self.OutVec`) (0.0 0.0 1.0)) (* (`self.WallRunSpeed`) Direction)) true false)
      (return true)
      (else
        _)))
  (return false))

(fn `WallRunUpdate `
  (bind _onwall_ (`self.WallRunMovement` (`Actor.K2_GetActorLocation` (`self.Character REF`)) (`self.WallRunEndVector`) -1.0))
  (if _onwall_
    (bind _output_get (set `self.WallRunnig?` true))
    (set `self.WallRunnig?Right` _output_get)
    (set `self.WallRunnig?Left` false)
    (set `CharacterMovementComponent.GravityScale` (`KismetMathLibrary.FInterpTo` (`CharacterMovementComponent.GravityScale` (`self.Character Movement`)) (`self.WallRungTargetGravity`) (`GameplayStatics.GetWorldDeltaSeconds`) 10.0) (`self.Character Movement`) :!label _label)
    (elif (`self.WallRunnig?Right`)
      (`self.WallRunEnd` 1.0)
      (else
        (bind _onwall__2 (`self.WallRunMovement` (`Actor.K2_GetActorLocation` (`self.Character REF`)) (`.left` (`self.WallRunEndVector`)) 1.0))
        (if _onwall__2
          (set `self.WallRunnig?` true)
          (set `self.WallRunnig?Right` false)
          (set `self.WallRunnig?Left` true)
          (goto _label)
          (else
            (`self.WallRunEnd` 1.0)))))))