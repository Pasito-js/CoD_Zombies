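; Health component Blueprint that tracks current and maximum health for the player and other actors.
; HealthRemove clamps damage, returning death state except on non-enemy player hits, which only play a land shake with the passed scale.
; Enemy hits on the player trigger a hit shake, HUD hit indicator and character AfterTakingDamage.
; HealthAdd writes its clamped sum to HealthMax, leaving HealthCurrent unchanged.
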(fn `HealthAdd`
  (params (Damage :type "Float (double-precision)"))
  (set `self.HealthMax` (`KismetMathLibrary.FClamp` (+ (`self.HealthCurrent`) Damage) 0.0 (`self.HealthMax`))))

(fn `HealthRemove`
  (params (Damage :type "Float (double-precision)") (Scale :type "Float (double-precision)") (`IsPlayer?` :type Boolean) (`NotEnemyHit?` :type Boolean) (EnemyREF :type "Actor Object Reference"))
  (returns (`IsDead?` :type Boolean))
  (bind _output_get (set `self.HealthCurrent` (`KismetMathLibrary.FClamp` (- (`self.HealthCurrent`) Damage) 0.0 (`self.HealthMax`))))
  (if `IsPlayer?`
    (`PlayerController.ClientStartCameraShake` :`self` (`GameplayStatics.GetPlayerController` 0) :`Shake` (select `bool` `NotEnemyHit?` :`false` "/Game/_Main/Blueprints/CameraShake/BP_CameraShakeOnHit.BP_CameraShakeOnHit_C" :`true` "/Game/_Main/Blueprints/CameraShake/BP_CameraShakeOnLand.BP_CameraShakeOnLand_C" :!type "CameraShakeBase Class Reference") :`Scale` (`KismetMathLibrary.SelectFloat` Scale 1.0 `NotEnemyHit?`))
    (if (not `NotEnemyHit?`)
      (bind _foundwidgets (`WidgetBlueprintLibrary.GetAllWidgetsOfClass` "/Game/_Main/Widgets/WBP_PlayerHUD.WBP_PlayerHUD_C"))
      (`/Game/_Main/Widgets/WBP_PlayerHUD.HitIndicator` (`|GetArrayItem` _foundwidgets) EnemyREF)
      (bind _asbp_first_person_character (cast `/Game/_Main/Blueprints/Characters/BP_FirstPersonCharacter` (`GameplayStatics.GetPlayerCharacter` 0)))
      (bind _returnvalue (<= _output_get 0.0))
      (`/Game/_Main/Blueprints/Characters/BP_FirstPersonCharacter.AfterTakingDamage` _asbp_first_person_character _returnvalue)
      (return _returnvalue))
    (else
      (return _returnvalue))))