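; Wall-mounted weapon buy that gives the player a weapon or refills ammo for a slot when interacted with.
; On BeginPlay it loads the mesh from DT_Weapon by WeaponIndex and paints all its materials white.
; A short sphere trace snaps it to the nearby surface, offset along and facing the hit normal.
; Interaction functions report price and weapon index, while the character handles the weapon or ammo grant.
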(event `self.ReceiveBeginPlay`
  (bind _weapon_skm (`self.Weapon_SKM`))
  (bind _returnvalue (`SceneComponent.K2_GetComponentLocation` (`self.DefaultSceneRoot`)))
  (bind _returnvalue_2 (`|GetDataTableRow` "/Game/_Main/Blueprints/DataTables/DT_Weapon.DT_Weapon" (`KismetStringLibrary.Conv_StringToName` (`KismetStringLibrary.Conv_IntToString` (`self.WeaponIndex`))))
    (:`then`
      (`SkeletalMeshComponent.SetSkeletalMeshAsset` (`self.Weapon_SKM`) (break `/Game/_Main/Blueprints/Structures/S_Weapon` _returnvalue_2))
      (bind _outhit (`KismetSystemLibrary.SphereTraceSingle` _returnvalue (+ _returnvalue (1.0 1.0 1.0)) 30.0 "TraceTypeQuery1"))
      (bind _returnvalue_3 (`KismetMathLibrary.Conv_VectorToRotator` (`.Normal` (`GameplayStatics.BreakHitResult` _outhit))))
      (`SceneComponent.K2_SetWorldTransform` (`self.DefaultSceneRoot`) (`KismetMathLibrary.MakeTransform` (+ (`.ImpactPoint` (`GameplayStatics.BreakHitResult` _outhit)) (* (`KismetMathLibrary.GetForwardVector` _returnvalue_3) 5.0)) _returnvalue_3) false false)
      (for _index (range (`PrimitiveComponent.GetNumMaterials` _weapon_skm))
        (`PrimitiveComponent.SetMaterial` _weapon_skm _index "/Game/_Main/Materials/White.White")))))

(event `/Game/_Main/Blueprints/Interfaces/BPI_Inreraction.OnInteract`
  (params (Ammo :type Boolean) (AmmoSlot :type Integer))
  (if (not Ammo)
    (bind _asbp_first_person_character (cast `/Game/_Main/Blueprints/Characters/BP_FirstPersonCharacter` (`GameplayStatics.GetPlayerCharacter` 0)))
    (`/Game/_Main/Blueprints/Characters/BP_FirstPersonCharacter.Set New Weapon To Slot` _asbp_first_person_character (`self.WeaponIndex`))
    (else
      (bind _asbp_first_person_character_2 (cast `/Game/_Main/Blueprints/Characters/BP_FirstPersonCharacter` (`GameplayStatics.GetPlayerCharacter` 0)))
      (`/Game/_Main/Blueprints/Characters/BP_FirstPersonCharacter.SetMaxAmmo` _asbp_first_person_character_2 AmmoSlot))))

(fn `CanInteract`
  (returns (CanInteract :type Boolean) (NeedPower :type Boolean))
  (return false false))

(fn `Is Interectable / Get Details`
  (returns (Type :type "/Game/_Main/Blueprints/Enums/E_Interaction Enum") (Text :type Text) (Price :type Integer) (WeaponIndex :type Integer))
  (return "NewEnumerator2" "" (`self.Price`) (`self.WeaponIndex`)))

(fn `UserConstructionScript`)