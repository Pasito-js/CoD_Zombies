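; Boarded-up window barricade that zombies tear down and the player rebuilds through interaction for points.
; Five planks get jittered transforms at BeginPlay, then slide out or back on timelines, tracked by a per-plank state array.
; Removal and rebuilding each pick a random eligible plank and mark it busy before animating.
; Selector functions set the nearest living overlapping zombie's blackboard WalkingState for plank removal or vaulting.
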(event `RemovePlank1`
  (bind _plank1 (`self.Plank1`))
  (bind _output_location (`KismetMathLibrary.BreakTransform` (`|GetArrayItem` (`self.PlanksTransform`))))
  (bind (_direction _alpha) (`Timeline|PullPlankTL` :!via `PlayFromStart`)
    (:`Update`
      (`SceneComponent.K2_SetRelativeLocation` (`self.Plank1`) (`KismetMathLibrary.VLerp` _output_location (- _output_location (0.0 100.0 0.0)) _alpha) false false))
    (:`Finished`
      (`SceneComponent.SetVisibility` _plank1 false false)
      (`PrimitiveComponent.SetCollisionEnabled` _plank1 "NoCollision")
      (`KismetArrayLibrary.Array_Set` (`self.PlankState`) 0 "NewEnumerator2"))))

(event `self.ReceiveBeginPlay`
  (`self.Set Plank to Array`)
  (`self.Randomise Plank Transform`))

(event `Can Remove Plank Check`
  (params (`Zombies REF` :type "/Game/_Main/Blueprints/Characters/Zombie/BP_EnemyMain Object Reference"))
  (if (<= (`self.Planks removing  Now`) 3)
    (`/Engine/EditorBlueprintResources/StandardMacros.DoOnce` false :!label _label
      (:`Completed`
        (`self.Calculate Removable Plank` `Zombies REF`)))))

(event `Reset Zombie Plank Checker`
  (goto _label :!via `Reset`))

(event `RemovePlank2`
  (bind _plank2 (`self.Plank2`))
  (bind _output_location (`KismetMathLibrary.BreakTransform` (`|GetArrayItem` (`self.PlanksTransform`) 1)))
  (bind (_direction _alpha) (`Timeline|Timeline` :!via `PlayFromStart`)
    (:`Update`
      (`SceneComponent.K2_SetRelativeLocation` (`self.Plank2`) (`KismetMathLibrary.VLerp` _output_location (- _output_location (0.0 100.0 0.0)) _alpha) false false))
    (:`Finished`
      (`SceneComponent.SetVisibility` _plank2 false false)
      (`PrimitiveComponent.SetCollisionEnabled` _plank2 "NoCollision")
      (`KismetArrayLibrary.Array_Set` (`self.PlankState`) 1 "NewEnumerator2"))))

(event `AddPlank`
  (bind _output_location (`KismetMathLibrary.BreakTransform` (`|GetArrayItem` (`self.PlanksTransform`) (`self.Add Plank Number`))))
  (bind _output_get (set `self.PlankAddREF` (`|GetArrayItem` (`self.PlankArray`) (`self.Add Plank Number`))))
  (`SceneComponent.SetVisibility` _output_get true false)
  (bind (_direction _alpha) (`Timeline|Timeline_3` :!via `PlayFromStart`)
    (:`Update`
      (`SceneComponent.K2_SetRelativeLocation` (`self.PlankAddREF`) (`KismetMathLibrary.VLerp` (- _output_location (0.0 100.0 0.0)) _output_location _alpha) false false))
    (:`Finished`
      (bind _foundwidgets (`WidgetBlueprintLibrary.GetAllWidgetsOfClass` "/Game/_Main/Widgets/WBP_PlayerHUD.WBP_PlayerHUD_C"))
      (`/Game/_Main/Widgets/WBP_PlayerHUD.IncreasePoints ` (`|GetArrayItem` _foundwidgets) 10)
      (`KismetArrayLibrary.Array_Set` (`self.PlankState`) (`self.Add Plank Number`) "NewEnumerator0")
      (`KismetSystemLibrary.Delay` 1.0)
      (set `self.AddingPlank` false))))

(event `/Game/_Main/Blueprints/Interfaces/BPI_Inreraction.OnInteract`
  (params (Ammo :type Boolean) (AmmoSlot :type Integer))
  (set `self.AddingPlank` true)
  (`self.Calculate Add Planks`))

(event `RemovePlank3`
  (bind _plank3 (`self.Plank3`))
  (bind _output_location (`KismetMathLibrary.BreakTransform` (`|GetArrayItem` (`self.PlanksTransform`) 2)))
  (bind (_direction _alpha) (`Timeline|Timeline_0` :!via `PlayFromStart`)
    (:`Update`
      (`SceneComponent.K2_SetRelativeLocation` (`self.Plank3`) (`KismetMathLibrary.VLerp` _output_location (- _output_location (0.0 100.0 0.0)) _alpha) false false))
    (:`Finished`
      (`SceneComponent.SetVisibility` _plank3 false false)
      (`PrimitiveComponent.SetCollisionEnabled` _plank3 "NoCollision")
      (`KismetArrayLibrary.Array_Set` (`self.PlankState`) 2 "NewEnumerator2"))))

(event `RemovePlank4`
  (bind _plank4 (`self.Plank4`))
  (bind _output_location (`KismetMathLibrary.BreakTransform` (`|GetArrayItem` (`self.PlanksTransform`) 3)))
  (bind (_direction _alpha) (`Timeline|Timeline_2` :!via `PlayFromStart`)
    (:`Update`
      (`SceneComponent.K2_SetRelativeLocation` (`self.Plank4`) (`KismetMathLibrary.VLerp` _output_location (- _output_location (0.0 100.0 0.0)) _alpha) false false))
    (:`Finished`
      (`SceneComponent.SetVisibility` _plank4 false false)
      (`PrimitiveComponent.SetCollisionEnabled` _plank4 "NoCollision")
      (`KismetArrayLibrary.Array_Set` (`self.PlankState`) 3 "NewEnumerator2"))))

(event `RemovePlank5`
  (bind _plank5 (`self.Plank5`))
  (bind _output_location (`KismetMathLibrary.BreakTransform` (`|GetArrayItem` (`self.PlanksTransform`) 4)))
  (bind (_direction _alpha) (`Timeline|Timeline_1` :!via `PlayFromStart`)
    (:`Update`
      (`SceneComponent.K2_SetRelativeLocation` (`self.Plank5`) (`KismetMathLibrary.VLerp` _output_location (- _output_location (0.0 100.0 0.0)) _alpha) false false))
    (:`Finished`
      (`SceneComponent.SetVisibility` _plank5 false false)
      (`PrimitiveComponent.SetCollisionEnabled` _plank5 "NoCollision")
      (`KismetArrayLibrary.Array_Set` (`self.PlankState`) 4 "NewEnumerator2"))))

(fn `Calculate Add Planks`
  (locals (Zombier_REF :type "/Game/_Main/Blueprints/Characters/Zombie/BP_EnemyMain Object Reference") (`Check ` :type Boolean))
  (set `local.Check ` true)
  (for (_array_element _array_index) (`self.PlankState`) :!label _label
    (if (and (`|EnumEquality` _array_element "NewEnumerator2") (`local.Check `))
      (if (<= (`KismetMathLibrary.RandomFloatInRange` 0.0 1.0) 0.2)
        (set `local.Check ` false)
        (bind _output_get (set `self.Add Plank Number` _array_index))
        (`KismetArrayLibrary.Array_Set` (`self.PlankState`) _output_get "NewEnumerator1"))))
  (if (not (`local.Check `))
    (`self.AddPlank`)
    (else
      (goto _label))))

(fn `Calculate Avaible Planks Remove Zombies`
  (returns (`Zombies Remove Plank ` :type "Array of /Game/_Main/Blueprints/Characters/Zombie/BP_EnemyMain Object Reference"))
  (`KismetArrayLibrary.Array_Clear` (`self.Zombies Remove Plank `))
  (bind _outactors (`GameplayStatics.GetAllActorsOfClass` "/Game/_Main/Blueprints/Characters/Zombie/BP_EnemyMain.BP_EnemyMain_C"))
  (for _array_element _outactors
    (if (and (> (`/Game/_Main/Blueprints/Components/BPC_Health.HealthCurrent` (`/Game/_Main/Blueprints/Characters/Zombie/BP_EnemyMain.BPC_Health` _array_element)) 0.0) (`PrimitiveComponent.IsOverlappingActor` (`self.BoxCollision`) _array_element) (not (`/Game/_Main/Blueprints/Characters/Zombie/BP_EnemyMain.RemovingPlank?` _array_element)))
      (`KismetArrayLibrary.Array_Add` (`self.Zombies Remove Plank `) _array_element)))
  (return (`self.Zombies Remove Plank `)))

(fn `Calculate Overlapping Alive Zombies`
  (returns (`Zombies OVerlapping Alive` :type "Array of /Game/_Main/Blueprints/Characters/Zombie/BP_EnemyMain Object Reference"))
  (`KismetArrayLibrary.Array_Clear` (`self.Zombies OVerlapping Alive`))
  (bind _outactors (`GameplayStatics.GetAllActorsOfClass` "/Game/_Main/Blueprints/Characters/Zombie/BP_EnemyMain.BP_EnemyMain_C"))
  (for _array_element _outactors
    (if (and (> (`/Game/_Main/Blueprints/Components/BPC_Health.HealthCurrent` (`/Game/_Main/Blueprints/Characters/Zombie/BP_EnemyMain.BPC_Health` _array_element)) 0.0) (`PrimitiveComponent.IsOverlappingActor` (`self.BoxCollision`) _array_element))
      (`KismetArrayLibrary.Array_Add` (`self.Zombies OVerlapping Alive`) _array_element)))
  (return (`self.Zombies OVerlapping Alive`)))

(fn `Calculate Planks Off Window`
  (returns (`Planks Off Window ` :type "Float (double-precision)"))
  (locals (`Planks Off Window` :type "Float (double-precision)"))
  (set `local.Planks Off Window` 0.0)
  (for _array_element (`self.PlankState`)
    (if (`|EnumEquality` _array_element "NewEnumerator2")
      (`/Engine/EditorBlueprintResources/StandardMacros.IncrementFloat` (`local.Planks Off Window`))))
  (return (`local.Planks Off Window`)))

(fn `Calculate Planks On Window`
  (returns (`Planks On Window ` :type "Float (double-precision)"))
  (locals (`Planks On Window` :type "Float (double-precision)"))
  (set `local.Planks On Window` 0.0)
  (for _array_element (`self.PlankState`)
    (if (`|EnumEquality` _array_element "NewEnumerator0")
      (`/Engine/EditorBlueprintResources/StandardMacros.IncrementFloat` (`local.Planks On Window`))))
  (return (`local.Planks On Window`)))

(fn `Calculate Removable Plank`
  (params (ZombieREF :type "/Game/_Main/Blueprints/Characters/Zombie/BP_EnemyMain Object Reference"))
  (locals (Zombier_REF :type "/Game/_Main/Blueprints/Characters/Zombie/BP_EnemyMain Object Reference") (`Check ` :type Boolean))
  (set `local.Zombier_REF` ZombieREF)
  (`/Engine/EditorBlueprintResources/StandardMacros.IncrementInt` (`self.Planks removing  Now`)
    (:`  `
      (set `/Game/_Main/Blueprints/Characters/Zombie/BP_EnemyMain.RemovingPlank?` true (`local.Zombier_REF`))
      (set `local.Check ` true)
      (for (_array_element _array_index) (`self.PlankState`) :!label _label
        (if (and (`|EnumEquality` _array_element "NewEnumerator0") (`local.Check `))
          (if (<= (`KismetMathLibrary.RandomFloatInRange` 0.0 1.0) 0.2)
            (set `local.Check ` false)
            (bind _output_get (set `self.Remove Plank Number` _array_index))
            (`KismetArrayLibrary.Array_Set` (`self.PlankState`) _output_get "NewEnumerator1"))))
      (if (not (`local.Check `))
        (`/Game/_Main/Blueprints/Characters/Zombie/BP_EnemyMain.RemovePlank` (`local.Zombier_REF`) (`self.Remove Plank Number`))
        (else
          (goto _label))))))

(fn `CanInteract`
  (returns (CanInteract :type Boolean) (NeedPower :type Boolean))
  (return false false))

(fn `Is Interectable / Get Details`
  (returns (Type :type "/Game/_Main/Blueprints/Enums/E_Interaction Enum") (Text :type Text) (Price :type Integer) (WeaponIndex :type Integer))
  (return (select `bool` (and (< (`self.Calculate Planks On Window`) 5.0) (> (`self.Calculate Planks Off Window`) 0.0) (not (`self.AddingPlank`))) :`false` "NewEnumerator4" :`true` "NewEnumerator1" :!type "/Game/_Main/Blueprints/Enums/E_Interaction Enum") "build window" 0 0))

(fn `Randomise Plank Transform`
  (locals (`Array Index` :type Integer))
  (bind _returnvalue (`KismetMathLibrary.RandomFloatInRange` -10.0 10.0))
  (for (_array_element _array_index) (`self.PlankArray`)
    (set `local.Array Index` _array_index)
    (bind _returnvalue_2 (`SceneComponent.GetRelativeTransform` _array_element))
    (bind (_relativerotation_roll _relativerotation_pitch) (`KismetMathLibrary.BreakRotator` (`SceneComponent.RelativeRotation` _array_element)))
    (`SceneComponent.K2_SetRelativeTransform` _array_element (`KismetMathLibrary.MakeTransform` (+ (.location _returnvalue_2) (`KismetMathLibrary.SelectVector` (`KismetMathLibrary.MakeVector` _returnvalue) (`KismetMathLibrary.MakeVector` 0.0 0.0 _returnvalue) (< _relativerotation_pitch -70.0))) (`KismetMathLibrary.MakeRotator` (.roll (.rotation _returnvalue_2)) (+ (.pitch (.rotation _returnvalue_2)) (`KismetMathLibrary.RandomFloatInRange` -10.0 10.0)) (.yaw (.rotation _returnvalue_2))) (.scale _returnvalue_2)) false false)
    (`KismetArrayLibrary.Array_Set` (`self.PlanksTransform`) (`local.Array Index`) (`SceneComponent.GetRelativeTransform` (`|GetArrayItem` (`self.PlankArray`) (`local.Array Index`))))))

(fn `Select Planks Removing Zombie`
  (if (!= (`self.Calculate Planks On Window`) 0.0)
    (bind _asbp_enemy_main (cast `/Game/_Main/Blueprints/Characters/Zombie/BP_EnemyMain` (`.ReturnValue` (`GameplayStatics.FindNearestActor` (`SceneComponent.K2_GetComponentLocation` (`self.WindowMiddlePoint`)) (`self.Calculate Avaible Planks Remove Zombies`)))))
    (`BlackboardComponent.SetValueAsEnum` (`AIBlueprintHelperLibrary.GetBlackboard` (`AIBlueprintHelperLibrary.GetAIController` _asbp_enemy_main)) "WalkingState" (enumliteral `/Game/_Main/Blueprints/Enums/E_ZombieWalkToMap` "NewEnumerator1"))))

(fn `Select Vaulting Zombies`
  (if (not (`self.Vaulting?`))
    (bind _asbp_enemy_main (cast `/Game/_Main/Blueprints/Characters/Zombie/BP_EnemyMain` (`.ReturnValue` (`GameplayStatics.FindNearestActor` (`SceneComponent.K2_GetComponentLocation` (`self.WindowMiddlePoint`)) (`self.Calculate Overlapping Alive Zombies`)))))
    (`BlackboardComponent.SetValueAsEnum` (`AIBlueprintHelperLibrary.GetBlackboard` (`AIBlueprintHelperLibrary.GetAIController` _asbp_enemy_main)) "WalkingState" (enumliteral `/Game/_Main/Blueprints/Enums/E_ZombieWalkToMap` "NewEnumerator2"))))

(fn `Set Plank to Array`
  (`|VariableSetRef` (`self.PlankArray`) (`|MakeArray` (`self.Plank1`) (`self.Plank2`) (`self.Plank3`) (`self.Plank4`) (`self.Plank5`))))

(fn `UserConstructionScript`)