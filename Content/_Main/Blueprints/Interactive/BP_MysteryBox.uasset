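; Zombies-style mystery box interactable that, once bought, offers a random weapon to take before it closes.
; Timelines animate lid, weapon and box materials, while SpinWeapon recursively cycles DT_Weapon meshes with growing delays, skipping two held weapons.
; CalculateTeddy uses spin count and chance to trigger a flying teddy, which disables the box and notifies GM_CoDZombies to relocate it.
; A sky beam fades in on enable, out on departure.
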(event `Set Mystery Box Enabled`
  (params (`First Box` :type Boolean))
  (set `self.First Box` `First Box`)
  (`KismetSystemLibrary.Delay` 2.0)
  (`GameplayStatics.PlaySoundAtLocation` (`KismetArrayLibrary.Array_Random` (`self.SoundSpawn`)) (`self.K2_GetActorLocation`) (struct) 1.0 1.0 0.0 "/Game/MilitaryWeapDark/Sound/Attenuation/WeaponShot_att.WeaponShot_att" null null null)
  (bind (_direction _alpha) (`Timeline|SkyLightFlashTL` :!via `PlayFromStart`)
    (:`Update`
      (`MeshComponent.SetScalarParameterValueOnMaterials` (`self.SkyLight`) "FadeAmount" (`KismetMathLibrary.Lerp` 0.0 1.0 _alpha))
      (if (>= (`TimelineComponent.GetPlaybackPosition` (`self.SkyLightFlashTL`)) 3.0)
        (`MeshComponent.SetScalarParameterValueOnMaterials` (`self.SkyLight`) "FadeAmount" (`KismetMathLibrary.Lerp` 0.0 (`self.Calculate SkyLight Fade`) _alpha))))
    (:`Finished`
      (set `self.Times Spun` 0)
      (`self.Set Box Color` true)
      (set `self.Mystery Box In use` true))))

(event `OpenBox`
  (`self.SpinWeapon`)
  (bind (_direction _alpha) (`Timeline|OpenBoxTL` :!via `PlayFromStart` :!label _label)
    (:`Update`
      (`SceneComponent.K2_SetRelativeRotation` (`self.top_scene`) (`KismetMathLibrary.RLerp` (struct) (struct :`Roll` -80.0) _alpha) false false)
      (`SceneComponent.K2_SetRelativeLocation` (`self.Weapon`) (`KismetMathLibrary.VLerp` (`KismetMathLibrary.MakeVector` (`self.WeaponX`)) (select `ETimelineDirection` _direction :`Forward` (`KismetMathLibrary.MakeVector` (`self.WeaponX`) 0.0 90.0) :`Backward` (`self.WeaponLoc`)) _alpha) false false))
    (:`Finished`
      (switch `ETimelineDirection` _direction
        (:`Backward`
          (if (`self.Spawn Teddy`)
            (set `self.Spawn Teddy` false)
            (else
              (set `self.InteractionType` "NewEnumerator3")
              (set `self.Can Interact` true)))
          (set `self.SpinLastWeapon Index` 0)
          (set `self.AmountRow` 0)
          (set `self.SpinIndex` 1)
          (`SceneComponent.SetVisibility` (`self.Weapon`) false false))))))

(event `CloseBox`
  (bind (_relativelocation_x _relativelocation_y _relativelocation_z) (`KismetMathLibrary.BreakVector` (`SceneComponent.RelativeLocation` (`self.Weapon`))))
  (set `self.WeaponLoc` (`KismetMathLibrary.MakeVector` (`self.WeaponX`) _relativelocation_y _relativelocation_z))
  (goto _label :!via `ReverseFromEnd`))

(event `self.ReceiveTick`
  (params (DeltaSeconds :type "Float (single-precision)"))
  (`self.SkyLight Opacity`))

(event `self.ReceiveBeginPlay`
  (`TimelineComponent.SetPlayRate` (`self.OpenBoxTL`) (/ 1.0 (`self.OpenTime`)))
  (`TimelineComponent.SetPlayRate` (`self.CloseSlowlyBoxTL`) (/ 1.0 (`self.CloseSlowlyTime`))))

(event `/Game/_Main/Blueprints/Interfaces/BPI_Inreraction.OnInteract`
  (params (Ammo :type Boolean) (AmmoSlot :type Integer))
  (if (`self.Can Interact`)
    (switch `/Game/_Main/Blueprints/Enums/E_Interaction` (`self.InteractionType`)
      (:`NewEnumerator1`
        (set `self.Can Interact` false)
        (set `self.InteractionType` "NewEnumerator4")
        (`SceneComponent.SetVisibility` (`self.Weapon`) false false)
        (bind _asbp_first_person_character (cast `/Game/_Main/Blueprints/Characters/BP_FirstPersonCharacter` (`GameplayStatics.GetPlayerCharacter` 0)))
        (`/Game/_Main/Blueprints/Characters/BP_FirstPersonCharacter.Set New Weapon To Slot` _asbp_first_person_character (`self.SpinLastWeapon Index`))
        (`self.CloseBox`))
      (:`NewEnumerator3`
        (set `self.Can Interact` false)
        (set `self.InteractionType` "NewEnumerator4")
        (`SceneComponent.SetVisibility` (`self.Weapon`) true false)
        (bind _asbp_first_person_character_2 (cast `/Game/_Main/Blueprints/Characters/BP_FirstPersonCharacter` (`GameplayStatics.GetPlayerCharacter` 0)))
        (set `self.As BP First Person Character` _asbp_first_person_character_2)
        (bind _weaponslots (`/Game/_Main/Blueprints/Characters/BP_FirstPersonCharacter.WeaponSlots` _asbp_first_person_character_2))
        (bind _output_indexweapon (break `/Game/_Main/Blueprints/Structures/S_WeaponSlot` (`|GetArrayItem` _weaponslots 1)))
        (set `self.WeaponIndex1` _output_indexweapon)
        (bind _output_indexweapon_2 (break `/Game/_Main/Blueprints/Structures/S_WeaponSlot` (`|GetArrayItem` _weaponslots 2)))
        (set `self.WeaponIndex2` _output_indexweapon_2)
        (bind _outrownames (`DataTableFunctionLibrary.GetDataTableRowNames` "/Game/_Main/Blueprints/DataTables/DT_Weapon.DT_Weapon"))
        (for _array_element _outrownames
          (`|GetDataTableRow` "/Game/_Main/Blueprints/DataTables/DT_Weapon.DT_Weapon" _array_element
            (:`then`
              (`/Engine/EditorBlueprintResources/StandardMacros.IncrementInt` (`self.AmountRow`)))))
        (`self.OpenBox`)))))

(event `SpinWeapon`
  (bind _spinshowweapon (`self.SpinShowWeapon`))
  (if (<= (`self.SpinIndex`) 50)
    (set `self.SpinShowWeapon` (`KismetMathLibrary.RandomIntegerInRange` 1 (`self.AmountRow`)))
    (if (and (!= _spinshowweapon (`self.WeaponIndex1`)) (!= _spinshowweapon (`self.WeaponIndex2`)) (!= _spinshowweapon (`self.SpinLastWeapon Index`)))
      (`KismetSystemLibrary.Delay` (/ (`KismetMathLibrary.FClamp` (- (`KismetMathLibrary.Conv_IntToDouble` (`self.SpinIndex`)) 20.0) 1.0 50.0) 100.0))
      (if (== (`self.SpinIndex`) 49)
        (`self.Calculate Teddy`)
        (if (`self.Spawn Teddy`)
          (`SceneComponent.SetVisibility` (`self.Weapon`) false false)
          (`SceneComponent.SetVisibility` (`self.Teddy`) true false)
          (`KismetSystemLibrary.Delay` 1.0)
          (`self.Set Teddy Flying`)
          (else
            (`/Engine/EditorBlueprintResources/StandardMacros.IncrementInt` (`self.Times Spun`)
              (:`  `
                (bind _returnvalue (`|GetDataTableRow` "/Game/_Main/Blueprints/DataTables/DT_Weapon.DT_Weapon" (`KismetStringLibrary.Conv_StringToName` (`KismetStringLibrary.Conv_IntToString` (`self.SpinShowWeapon`))) :!label _label_2)
                  (:`then`
                    (`SkeletalMeshComponent.SetSkeletalMeshAsset` (`self.Weapon`) (break `/Game/_Main/Blueprints/Structures/S_Weapon` _returnvalue))
                    (set `self.SpinLastWeapon Index` (`self.SpinShowWeapon`))
                    (`/Engine/EditorBlueprintResources/StandardMacros.IncrementInt` (`self.SpinIndex`)
                      (:`  `
                        (`self.SpinWeapon`)))))))))
        (else
          (goto _label_2)))
      (else
        (`self.SpinWeapon`)))
    (else
      (set `self.InteractionType` "NewEnumerator1")
      (set `self.Can Interact` true)
      (`self.CloseBoxSlowly`))))

(event `CloseBoxSlowly`
  (bind _weaponx (`self.WeaponX`))
  (bind (_direction _alpha) (`Timeline|CloseSlowlyBoxTL` :!via `PlayFromStart`)
    (:`Update`
      (`SceneComponent.K2_SetRelativeLocation` (`self.Weapon`) (`KismetMathLibrary.VLerp` (`KismetMathLibrary.MakeVector` _weaponx 0.0 90.0) (`KismetMathLibrary.MakeVector` _weaponx 0.0 60.0) _alpha) false false))
    (:`Finished`
      (if (`|EnumEquality` (`self.InteractionType`) "NewEnumerator1")
        (set `self.Can Interact` false)
        (set `self.InteractionType` "NewEnumerator4")
        (`self.CloseBox`)))))

(event `Set Teddy Flying`
  (bind _teddy (`self.Teddy`))
  (bind (_direction _alpha) (`Timeline|TeddyFlyingTL` :!via `PlayFromStart`)
    (:`Update`
      (`SceneComponent.K2_SetRelativeLocation` (`self.Teddy`) (`KismetMathLibrary.MakeVector` 0.0 0.0 _alpha) false false))
    (:`Finished`
      (`self.CloseBox`)
      (`self.Set Box Color` false)
      (bind _asgm_co_dzombies (cast `/Game/_Main/Blueprints/Game/GM_CoDZombies` (`GameplayStatics.GetGameMode`)))
      (`/Game/_Main/Blueprints/Game/GM_CoDZombies.Set Location Mystery Box` _asgm_co_dzombies false)
      (bind (_direction_2 _alpha_2) (`Timeline|SkyLightFadeAwayTL` :!via `PlayFromStart`)
        (:`Update`
          (`MeshComponent.SetScalarParameterValueOnMaterials` (`self.SkyLight`) "FadeAmount" (`KismetMathLibrary.Lerp` (`self.Calculate SkyLight Fade`) 0.0 _alpha_2)))
        (:`Finished`
          (set `self.Mystery Box In use` false)
          (`SceneComponent.SetVisibility` _teddy false false)
          (`SceneComponent.K2_SetRelativeLocation` _teddy (0.0 0.0 70.0) false false))))))

(event `Set Box Color`
  (params (Enabled :type Boolean))
  (if Enabled
    (bind (_direction _alpha) (`Timeline|Set Box Color TL` :!via `PlayFromStart` :!label _label_3)
      (:`Update`
        (`MeshComponent.SetScalarParameterValueOnMaterials` (`self.Top`) "Alpha" _alpha)
        (`MeshComponent.SetScalarParameterValueOnMaterials` (`self.Bottom`) "Alpha" _alpha)
        (`MeshComponent.SetScalarParameterValueOnMaterials` (`self.Left`) "Alpha" _alpha)
        (`MeshComponent.SetScalarParameterValueOnMaterials` (`self.Right`) "Alpha" _alpha)
        (`MeshComponent.SetScalarParameterValueOnMaterials` (`self.Back`) "Alpha" _alpha)
        (`MeshComponent.SetScalarParameterValueOnMaterials` (`self.Front`) "Alpha" _alpha))
      (:`Finished`
        (switch `ETimelineDirection` _direction
          (:`Forward`
            (set `self.Can Interact` true)
            (set `self.InteractionType` "NewEnumerator3")))))
    (else
      (goto _label_3 :!via `ReverseFromEnd`))))

(fn `Calculate Teddy`
  (if (< (`self.Times Spun`) 4)
    (set `self.Spawn Teddy` true)
    (elif (< (`self.Times Spun`) 8)
      (if (and (== (`self.Times Spun`) 7) (`self.FirstBox`))
        (set `self.Spawn Teddy` true)
        (elif (<= (`KismetMathLibrary.RandomFloatInRange` 0.0 1.0) 0.15)
          (set `self.Spawn Teddy` true)
          (else
            (set `self.Spawn Teddy` false))))
      (elif (< (`self.Times Spun`) 12)
        (if (<= (`KismetMathLibrary.RandomFloatInRange` 0.0 1.0) 0.3)
          (set `self.Spawn Teddy` true)
          (else
            (set `self.Spawn Teddy` false)))
        (elif (<= (`KismetMathLibrary.RandomFloatInRange` 0.0 1.0) 0.5)
          (set `self.Spawn Teddy` true)
          (else
            (set `self.Spawn Teddy` false)))))))

(fn `CanInteract`
  (returns (CanInteract :type Boolean) (NeedPower :type Boolean))
  (return (`self.Can Interact`) false))

(fn `Is Interectable / Get Details`
  (returns (Type :type "/Game/_Main/Blueprints/Enums/E_Interaction Enum") (Text :type Text) (Price :type Integer) (WeaponIndex :type Integer))
  (return (`self.InteractionType`) (select `/Game/_Main/Blueprints/Enums/E_Interaction` (`self.InteractionType`) :`NewEnumerator1` "Take" :`NewEnumerator3` "Open Mystery Box" :!type "Text") (`self.InteractionPrice`) (`self.SpinLastWeapon Index`)))

(fn `SkyLight Opacity`
  (if (`self.Mystery Box In use`)
    (if (`PrimitiveComponent.IsOverlappingActor` (`self.SkyLightCollision`) (`GameplayStatics.GetPlayerCharacter` 0))
      (`MeshComponent.SetScalarParameterValueOnMaterials` (`self.SkyLight`) "FadeAmount" (`self.Calculate SkyLight Fade`)))))

(fn `UserConstructionScript`
  (`MeshComponent.SetScalarParameterValueOnMaterials` (`self.SkyLight`) "FadeAmount" 0.0)
  (`MeshComponent.SetScalarParameterValueOnMaterials` (`self.Top`) "Alpha" 1.0)
  (`MeshComponent.SetScalarParameterValueOnMaterials` (`self.Bottom`) "Alpha" 1.0)
  (`MeshComponent.SetScalarParameterValueOnMaterials` (`self.Left`) "Alpha" 1.0)
  (`MeshComponent.SetScalarParameterValueOnMaterials` (`self.Right`) "Alpha" 1.0)
  (`MeshComponent.SetScalarParameterValueOnMaterials` (`self.Back`) "Alpha" 1.0)
  (`MeshComponent.SetScalarParameterValueOnMaterials` (`self.Front`) "Alpha" 1.0))