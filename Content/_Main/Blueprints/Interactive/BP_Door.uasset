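; BP_Door is an interactable door for a CoD Zombies-style mode, exposing a price, prompt text and power-requirement flag.
; On interact, it compares the player's distance to two side markers and flags the nearer side's room number as opened in GM_CoDZombies' spawn room array.
; It then disables further interaction, raises the door mesh along Z with a duration-scaled timeline, and destroys itself when finished.
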(event `/Game/_Main/Blueprints/Interfaces/BPI_Inreraction.OnInteract`
  (params (Ammo :type Boolean) (AmmoSlot :type Integer))
  (bind _returnvalue (`SceneComponent.K2_GetComponentLocation` (`Character.CapsuleComponent` (`GameplayStatics.GetPlayerCharacter` 0))))
  (if (< (`KismetMathLibrary.Vector_Distance` _returnvalue (`SceneComponent.K2_GetComponentLocation` (`self.2`))) (`KismetMathLibrary.Vector_Distance` _returnvalue (`SceneComponent.K2_GetComponentLocation` (`self.1`))))
    (bind _asgm_co_dzombies (cast `/Game/_Main/Blueprints/Game/GM_CoDZombies` (`GameplayStatics.GetGameMode`)))
    (`KismetArrayLibrary.Array_Set` (`/Game/_Main/Blueprints/Game/GM_CoDZombies.SpawnRoomsOpened` _asgm_co_dzombies) (`self.Side2RoomNumber`) true true)
    (else
      (bind _asgm_co_dzombies_2 (cast `/Game/_Main/Blueprints/Game/GM_CoDZombies` (`GameplayStatics.GetGameMode`)))
      (`KismetArrayLibrary.Array_Set` (`/Game/_Main/Blueprints/Game/GM_CoDZombies.SpawnRoomsOpened` _asgm_co_dzombies_2) (`self.Side1RoomNumber`) true true)))
  (set `self.CanInteract ` false)
  (`self.OpenDoor`))

(event `OpenDoor`
  (bind (_relativelocation_x _relativelocation_y _relativelocation_z) (`KismetMathLibrary.BreakVector` (`SceneComponent.RelativeLocation` (`self.Door`))))
  (`TimelineComponent.SetPlayRate` (`self.OpenDoorTL`) (/ 1.0 (`self.OpeningTime`)))
  (set `self.StartLocation` (`SceneComponent.RelativeLocation` (`self.Door`)))
  (set `self.EndLocation` (`KismetMathLibrary.MakeVector` _relativelocation_x _relativelocation_y (+ _relativelocation_z (`self.OpeningZValue`))))
  (bind (_direction _newtrack_0) (`Timeline|OpenDoorTL` :!via `PlayFromStart`)
    (:`Update`
      (`SceneComponent.K2_SetRelativeLocation` (`self.Door`) (`KismetMathLibrary.VLerp` (`self.StartLocation`) (`self.EndLocation`) _newtrack_0) false false))
    (:`Finished`
      (`self.K2_DestroyActor`))))

(fn `CanInteract`
  (returns (CanInteract :type Boolean) (NeedPower :type Boolean))
  (return (`self.CanInteract `) (`self.NeewPower`)))

(fn `Is Interectable / Get Details`
  (returns (Type :type "/Game/_Main/Blueprints/Enums/E_Interaction Enum") (Text :type Text) (Price :type Integer) (WeaponIndex :type Integer))
  (return "NewEnumerator3" (`self.InteractText`) (`self.Price`) 0))

(fn `UserConstructionScript`)