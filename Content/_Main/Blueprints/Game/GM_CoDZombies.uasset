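; Game mode for a CoD Zombies-style wave game that creates the HUD, runs rounds and places the mystery box.
; Each round scales zombie count, health, attack and movement speeds, then a looping timer spawns walkers or runners up to an alive cap.
; Spawners in opened rooms and a new box location are picked randomly, retrying until one succeeds.
; CheckIfRoundEnd advances the round once all zombies have spawned and none remain alive.
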(event `self.ReceiveBeginPlay`
  (bind _returnvalue (`|CreateWidget` "/Game/_Main/Widgets/WBP_PlayerHUD.WBP_PlayerHUD_C"))
  (`UserWidget.AddToViewport` _returnvalue 0)
  (`self.IncreaseRound`)
  (`self.Set Mystery Box Numbers`)
  (`self.Set Location Mystery Box` true))

(event `IncreaseRound`
  ;[1 1 1] Increase Round
  (`self.SetMaxHealth`)
  (`/Engine/EditorBlueprintResources/StandardMacros.IncrementInt` (`self.RoundNumber`)
    (:`  `
      (`KismetSystemLibrary.Delay` (`self.RoundBetweenTime`))
      (bind _foundwidgets (`WidgetBlueprintLibrary.GetAllWidgetsOfClass` "/Game/_Main/Widgets/WBP_PlayerHUD.WBP_PlayerHUD_C"))
      (`/Game/_Main/Widgets/WBP_PlayerHUD.IncreaseRound` (`|GetArrayItem` _foundwidgets))
      (`self.StartRound`))))

(event `StartRound`
  (bind _roundnumber (`self.RoundNumber`))
  ;[1 1 1] RoundSystem
  (set `self.TotalZombiesInRound` (`KismetMathLibrary.SelectInt` (`KismetMathLibrary.Round` (* (* (`self.RoundNumber`) 0.15) (`self.maxZombieInLevel`))) (`KismetMathLibrary.SelectInt` 6 9 (== _roundnumber 1)) (> _roundnumber 2)))
  (`self.SetWalk/RunSpeed`)
  (`self.SetAttackSpeed`)
  (`KismetSystemLibrary.Delay` 0.2)
  (bind _returnvalue (`KismetSystemLibrary.K2_SetTimerDelegate` (delegate `SpawnZombie`) (`self.SpawnBetweenTime`) true)))

(event `SpawnZombie`
  ;[1 1 1] RoundSystem
  (if (< (`self.ZombeisSpawned`) (`self.TotalZombiesInRound`))
    (if (<= (`self.ZombiesAlived`) (`self.maxZombieInLevel`))
      (`self.Set If walker / runner`)
      (`self.CheckSpawnLocationAndSpawn`)
      (`/Engine/EditorBlueprintResources/StandardMacros.IncrementInt` (`self.ZombeisSpawned`)
        (:`  `
          (`/Engine/EditorBlueprintResources/StandardMacros.IncrementInt` (`self.ZombiesAlived`)))))
    (else
      (`KismetSystemLibrary.K2_ClearAndInvalidateTimerHandle` (stale `StartRound` _returnvalue) :!label _label))))

(event `CheckIfRoundEnd`
  ;[1 1 1] RoundSystem
  (`KismetSystemLibrary.Delay` 0.1)
  (if (and (>= (`self.ZombeisSpawned`) (`self.TotalZombiesInRound`)) (== (`self.ZombiesAlived`) 0))
    (set `self.ZombeisSpawned` 0)
    (set `self.RunnersSpawned` 0)
    (`self.IncreaseRound`)
    (goto _label)))

(fn `CheckSpawnLocationAndSpawn`
  (locals (Spawned :type Boolean) (SpawnsOpen :type "Float (double-precision)") (ArrayElement :type "/Game/_Main/Blueprints/Game/BP_ZombieSpawner Object Reference"))
  (set `local.Spawned` false)
  (set `local.SpawnsOpen` 0.0)
  (bind _outactors (`GameplayStatics.GetAllActorsOfClass` "/Game/_Main/Blueprints/Game/BP_ZombieSpawner.BP_ZombieSpawner_C"))
  (for _array_element _outactors
    (if (`|GetArrayItem` (`self.SpawnRoomsOpened`) (`/Game/_Main/Blueprints/Game/BP_ZombieSpawner.SpawnerRoomNumber` _array_element))
      (`/Engine/EditorBlueprintResources/StandardMacros.IncrementFloat` (`local.SpawnsOpen`))))
  (bind _outactors_2 (`GameplayStatics.GetAllActorsOfClass` "/Game/_Main/Blueprints/Game/BP_ZombieSpawner.BP_ZombieSpawner_C" :!label _label))
  (for _array_element_2 _outactors_2
    (set `local.ArrayElement` _array_element_2)
    (if (not (`local.Spawned`))
      (if (`|GetArrayItem` (`self.SpawnRoomsOpened`) (`/Game/_Main/Blueprints/Game/BP_ZombieSpawner.SpawnerRoomNumber` (`local.ArrayElement`)))
        (if (<= (`KismetMathLibrary.RandomFloatInRange` 0.0 1.0) (/ 1.0 (`local.SpawnsOpen`)))
          (`/Game/_Main/Blueprints/Game/BP_ZombieSpawner.Spawn` (`local.ArrayElement`) (`self.MaxHealth`) (`self.AttackSpeed`) (`self.ZombieMaxWalk`))
          (set `local.Spawned` true)))))
  (if (not (`local.Spawned`))
    (goto _label)))

(fn `Set If walker / runner`
  (set `self.TotalRunnersInRound` (`KismetMathLibrary.Round` (* (`KismetMathLibrary.Conv_IntToDouble` (`self.TotalZombiesInRound`)) (/ (`self.RoundNumber`) 20))))
  (if (< (`self.RoundNumber`) 3)
    (set `self.ZombieMaxWalk` (`self.WalkSpeed`))
    (elif (< (`self.RunnersSpawned`) (`self.TotalRunnersInRound`))
      (if (<= (`KismetMathLibrary.RandomFloatInRange` 0.0 1.0) (/ (- (`self.TotalRunnersInRound`) (`self.RunnersSpawned`)) (- (`self.TotalZombiesInRound`) (`self.ZombeisSpawned`))))
        (set `self.ZombieMaxWalk` (`self.RunWalk`))
        (`/Engine/EditorBlueprintResources/StandardMacros.IncrementInt` (`self.RunnersSpawned`))
        (else
          (set `self.ZombieMaxWalk` (`self.WalkSpeed`) :!label _label)))
      (else
        (goto _label)))))

(fn `Set Location Mystery Box`
  (params (First :type Boolean))
  (locals (`First?` :type Boolean) (BoxesOnLevel :type "Float (double-precision)") (Set :type Boolean))
  (set `local.First?` First)
  (set `local.BoxesOnLevel` (`KismetMathLibrary.Conv_IntToDouble` (`self.MysteryBoxesTotalOnLevel`)))
  (bind _outactors (`GameplayStatics.GetAllActorsOfClass` "/Game/_Main/Blueprints/Interactive/BP_MysteryBox.BP_MysteryBox_C"))
  (for _array_element _outactors :!label _label
    (if (not (`local.Set`))
      (if (and (<= (`KismetMathLibrary.RandomFloatInRange` 0.0 1.0) (/ 1.0 (`local.BoxesOnLevel`))) (!= (`/Game/_Main/Blueprints/Interactive/BP_MysteryBox.MysteryBoxNumber` _array_element) (`self.Current Number Mystery Box`)))
        (set `self.Current Number Mystery Box` (`/Game/_Main/Blueprints/Interactive/BP_MysteryBox.MysteryBoxNumber` _array_element))
        (`/Game/_Main/Blueprints/Interactive/BP_MysteryBox.Set Mystery Box Enabled` _array_element (`local.First?`))
        (set `local.Set` true)
        (else
          (`/Engine/EditorBlueprintResources/StandardMacros.DecrementFloat` (`local.BoxesOnLevel`))))))
  (if (not (`local.Set`))
    (goto _label)))

(fn `Set Mystery Box Numbers`
  (set `self.MysteryBoxesTotalOnLevel` 0)
  (bind _outactors (`GameplayStatics.GetAllActorsOfClass` "/Game/_Main/Blueprints/Interactive/BP_MysteryBox.BP_MysteryBox_C"))
  (for (_array_element _array_index) _outactors
    (set `/Game/_Main/Blueprints/Interactive/BP_MysteryBox.MysteryBoxNumber` _array_index _array_element)
    (`/Engine/EditorBlueprintResources/StandardMacros.IncrementInt` (`self.MysteryBoxesTotalOnLevel`))))

(fn `SetAttackSpeed`
  (bind _roundnumber (`self.RoundNumber`))
  (bind _roundnumber_2 (`self.RoundNumber`))
  (set `self.AttackSpeed` (`KismetMathLibrary.FClamp` (select `bool` (`KismetMathLibrary.InRange_IntInt` _roundnumber_2 0 20) :`false` (select `bool` (`KismetMathLibrary.InRange_IntInt` _roundnumber 21 100) :`false` 1.4 :`true` (+ (* (- _roundnumber 20) 0.05) 1.0)) :`true` (+ (* _roundnumber_2 0.01) 0.8)) 0.8 1.4)))

(fn `SetMaxHealth`
  (set `self.MaxHealth` (`KismetMathLibrary.FClamp` (`KismetMathLibrary.SelectFloat` (+ (`self.MaxHealth`) 100.0) (* (`self.MaxHealth`) 1.1) (< (`self.RoundNumber`) 10)) 150.0 50000.0)))

(fn `SetWalk/RunSpeed`
  (bind _roundnumber (`self.RoundNumber`))
  (bind _roundnumber_2 (`self.RoundNumber`))
  (set `self.WalkSpeed` (`KismetMathLibrary.FClamp` (select `bool` (`KismetMathLibrary.InRange_IntInt` _roundnumber_2 0 20) :`false` 80.0 :`true` (+ (* _roundnumber_2 2.5) 30.0)) 30.0 80.0))
  (set `self.RunWalk` (`KismetMathLibrary.FClamp` (select `bool` (`KismetMathLibrary.InRange_IntInt` _roundnumber 0 30) :`false` 370.0 :`true` (+ (* _roundnumber 6.0) 190.0)) 200.0 370.0)))

(fn `UserConstructionScript`)