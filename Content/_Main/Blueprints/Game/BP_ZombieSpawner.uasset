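; Zombie spawner that creates a BP_EnemyMain at its own transform with slightly randomized scale.
; The Spawn event sets the enemy's health, attack speed and walk speed from caller inputs, then hands it a target window and inside point.
; GetWindowLocation counts BP_Windows sharing the spawner's WindowNumber, then randomly picks one in a second pass, which never breaks, so later windows can override earlier picks.
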(event `Spawn`
  (params (MaxHealth :type "Float (double-precision)") (AttackSpeed :type "Float (double-precision)") (`MaxWalk / Run Speed` :type "Float (double-precision)"))
  (bind (_returnvalue_location _returnvalue_rotation) (`KismetMathLibrary.BreakTransform` (`self.GetTransform`)))
  (bind _returnvalue (`KismetMathLibrary.RandomFloatInRange` 0.9 1.2))
  (`self.Get Window Location`)
  (bind _returnvalue_2 (`|SpawnActorFromClass` "/Game/_Main/Blueprints/Characters/Zombie/BP_EnemyMain.BP_EnemyMain_C" (`KismetMathLibrary.MakeTransform` _returnvalue_location _returnvalue_rotation (`KismetMathLibrary.MakeVector` _returnvalue _returnvalue (`KismetMathLibrary.RandomFloatInRange` 0.95 1.1))) "AdjustIfPossibleButAlwaysSpawn" "MultiplyWithRoot" null null))
  (bind _bpc_health (`/Game/_Main/Blueprints/Characters/Zombie/BP_EnemyMain.BPC_Health` _returnvalue_2))
  (bind _output_get (set `/Game/_Main/Blueprints/Components/BPC_Health.HealthCurrent` MaxHealth _bpc_health))
  (set `/Game/_Main/Blueprints/Components/BPC_Health.HealthMax` _output_get _bpc_health)
  (set `/Game/_Main/Blueprints/Characters/Zombie/BP_EnemyMain.AttackSpeed` AttackSpeed _returnvalue_2)
  (set `CharacterMovementComponent.MaxWalkSpeed` `MaxWalk / Run Speed` (`Character.CharacterMovement` _returnvalue_2))
  (set `/Game/_Main/Blueprints/Characters/Zombie/BP_EnemyMain.WindowREF` (`self.WindowREF`) _returnvalue_2)
  (set `/Game/_Main/Blueprints/Characters/Zombie/BP_EnemyMain.WindowLocation` (`self.WindowLocation`) _returnvalue_2))

(fn `Get Window Location`
  (set `self.PossibleWindows` 0.0)
  (bind _outactors (`GameplayStatics.GetAllActorsOfClass` "/Game/_Main/Blueprints/Interactive/BP_Window.BP_Window_C"))
  (for _array_element _outactors
    (if (== (`/Game/_Main/Blueprints/Interactive/BP_Window.WindowNumber` _array_element) (`self.WindowNumber`))
      (`/Engine/EditorBlueprintResources/StandardMacros.IncrementFloat` (`self.PossibleWindows`))))
  (bind _outactors_2 (`GameplayStatics.GetAllActorsOfClass` "/Game/_Main/Blueprints/Interactive/BP_Window.BP_Window_C"))
  (for _array_element_2 _outactors_2
    (if (== (`/Game/_Main/Blueprints/Interactive/BP_Window.WindowNumber` _array_element_2) (`self.WindowNumber`))
      (if (<= (`KismetMathLibrary.RandomFloatInRange` 0.0 1.0) (/ 1.0 (`self.PossibleWindows`)))
        (set `self.WindowREF` _array_element_2)
        (set `self.WindowLocation` (`SceneComponent.K2_GetComponentLocation` (`/Game/_Main/Blueprints/Interactive/BP_Window.WindowInsidePoint` _array_element_2)))
        (else
          (`/Engine/EditorBlueprintResources/StandardMacros.DecrementFloat` (`self.PossibleWindows`)))))))

(fn `UserConstructionScript`)