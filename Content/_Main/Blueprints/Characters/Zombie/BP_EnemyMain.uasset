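; Base zombie enemy for a CoD Zombies-style round mode: it pulls planks from windows, vaults inside and attacks the player.
; Window entry chains an AI move (timeline-lerp fallback on failure), a timed rotation and a montage-synced vault with collision off.
; Damage uses DT_BoneHit bone multipliers or fixed knife damage.
; Death ragdolls the mesh, sets the blackboard Dead key, updates the game mode's round count and fades materials before destroying.
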(event `self.HitAttackCollision.OnComponentBeginOverlap`
  (params (OverlappedComponent :type "PrimitiveComponent Object Reference") (OtherActor :type "Actor Object Reference") (OtherComp :type "PrimitiveComponent Object Reference") (OtherBodyIndex :type Integer) (bFromSweep :type Boolean) (SweepResult :type "HitResult Structure (by ref)"))
  (if (`self.CanDamage?`)
    (bind _asbp_first_person_character (cast `/Game/_Main/Blueprints/Characters/BP_FirstPersonCharacter` OtherActor))
    (set `self.CanDamage?` false)
    (`/Game/_Main/Blueprints/Components/BPC_Health.HealthRemove` (`/Game/_Main/Blueprints/Characters/BP_FirstPersonCharacter.BPC_Health` _asbp_first_person_character) 25.0 0.0 true false self)))

(event `DeadFade`
  (bind (_direction _alpha) (`Timeline|DeadFadeTL` :!via `PlayFromStart`)
    (:`Update`
      (`MaterialInstanceDynamic.SetScalarParameterValue` (`self.DynamicMaterial`) "Fade" _alpha)
      (`MaterialInstanceDynamic.SetScalarParameterValue` (`self.DynamicMaterial1`) "Fade" _alpha))
    (:`Finished`
      (`self.K2_DestroyActor`))))

(event `self.ReceiveTick`
  (params (DeltaSeconds :type "Float (single-precision)"))
  (`self.AttackRotation`))

(event `RemovePlank`
  (params (`Remove Plank Number` :type Integer))
  (bind _windowref (`self.WindowREF`))
  (bind _windowref_2 (`self.WindowREF`))
  (bind (_returnvalue_roll _returnvalue_pitch _returnvalue_yaw) (`KismetMathLibrary.BreakRotator` (`KismetMathLibrary.FindLookAtRotation` (`SceneComponent.K2_GetComponentLocation` (`self.CapsuleComponent`)) (`SceneComponent.K2_GetComponentLocation` (`/Game/_Main/Blueprints/Interactive/BP_Window.WindowMiddlePoint` (`self.WindowREF`))))))
  (set `self.Remove Plank Number` `Remove Plank Number`)
  (`SceneComponent.K2_SetWorldRotation` (`self.CapsuleComponent`) (`KismetMathLibrary.MakeRotator` 0.0 0.0 _returnvalue_yaw) false false)
  (`|PlayMontage` (`self.Mesh`) "/Game/_Main/Blueprints/Characters/Zombie/Animation/AnimMontages/AM_PullPlank.AM_PullPlank"
    (:`then`
      (`KismetSystemLibrary.Delay` 0.5)
      (`/Engine/EditorBlueprintResources/StandardMacros.DecrementInt` (`/Game/_Main/Blueprints/Interactive/BP_Window.Planks removing  Now` _windowref)
        (:`  `
          (`/Game/_Main/Blueprints/Interactive/BP_Window.Reset Zombie Plank Checker` _windowref)
          (`KismetSystemLibrary.Delay` 0.3)
          (if (> (`/Game/_Main/Blueprints/Components/BPC_Health.HealthCurrent` (`self.BPC_Health`)) 0.0)
            (switch `int` (`self.Remove Plank Number`)
              (:`0`
                (`/Game/_Main/Blueprints/Interactive/BP_Window.RemovePlank1` _windowref_2))
              (:`1`
                (`/Game/_Main/Blueprints/Interactive/BP_Window.RemovePlank2` _windowref_2))
              (:`2`
                (`/Game/_Main/Blueprints/Interactive/BP_Window.RemovePlank3` _windowref_2))
              (:`3`
                (`/Game/_Main/Blueprints/Interactive/BP_Window.RemovePlank4` _windowref_2))
              (:`4`
                (`/Game/_Main/Blueprints/Interactive/BP_Window.RemovePlank5` _windowref_2)))
            (`KismetSystemLibrary.Delay` 1.05)
            (set `self.RemovingPlank?` false)
            (else
              (`KismetArrayLibrary.Array_Set` (`/Game/_Main/Blueprints/Interactive/BP_Window.PlankState` (`self.WindowREF`)) (`self.Remove Plank Number`) "NewEnumerator0"))))))))

(event `Move To Vaulting Position`
  (bind _windowref (`self.WindowREF`))
  (bind (_vaultstarttransform_location _vaultstarttransform_rotation _vaultstarttransform_scale) (`KismetMathLibrary.BreakTransform` (`self.VaultStartTransform`)))
  (bind (_returnvalue_location _returnvalue_rotation) (`KismetMathLibrary.BreakTransform` (`SceneComponent.K2_GetComponentToWorld` (`self.CapsuleComponent`))))
  (bind _returnvalue_location_2 (`KismetMathLibrary.BreakTransform` (`SceneComponent.K2_GetComponentToWorld` (`/Game/_Main/Blueprints/Interactive/BP_Window.WindowInsidePoint` _windowref))))
  (bind (_returnvalue_location_3 _returnvalue_rotation_2) (`KismetMathLibrary.BreakTransform` (`SceneComponent.K2_GetComponentToWorld` (`/Game/_Main/Blueprints/Interactive/BP_Window.WindowInsidePoint` (`self.WindowREF`)))))
  (set `/Game/_Main/Blueprints/Interactive/BP_Window.Vaulting?` true _windowref)
  (`|AIMoveTo` self _returnvalue_location_2 null 10.0
    (:`OnSuccess`
      (`/Engine/EditorBlueprintResources/StandardMacros.DoOnce` false :!label _label
        (:`Completed`
          (`self.RotateToWindow`))))
    (:`OnFail`
      (`self.Calcucate Force Move TL`)
      (set `self.VaultStartTransform` (`KismetMathLibrary.MakeTransform` _returnvalue_location _returnvalue_rotation (`SceneComponent.K2_GetComponentScale` (`self.Mesh`))))
      (bind (_direction _alpha) (`Timeline|ForceMoveTL` :!via `PlayFromStart`)
        (:`Update`
          (`SceneComponent.K2_SetWorldTransform` (`self.CapsuleComponent`) (`KismetMathLibrary.TLerp` (`self.VaultStartTransform`) (`KismetMathLibrary.MakeTransform` _returnvalue_location_3 _returnvalue_rotation_2 _vaultstarttransform_scale) _alpha) false false))
        (:`Finished`
          (goto _label))))))

(event `RotateToWindow`
  (bind (_returnvalue_roll _returnvalue_pitch _returnvalue_yaw) (`KismetMathLibrary.BreakRotator` (`SceneComponent.K2_GetComponentRotation` (`self.CapsuleComponent`))))
  (bind (_returnvalue_roll_2 _returnvalue_pitch_2 _returnvalue_yaw_2) (`KismetMathLibrary.BreakRotator` (`SceneComponent.K2_GetComponentRotation` (`/Game/_Main/Blueprints/Interactive/BP_Window.WindowMiddlePoint` (`self.WindowREF`)))))
  (bind _returnvalue (- _returnvalue_yaw _returnvalue_yaw_2))
  (`TimelineComponent.SetPlayRate` (`self.RotateToWindowTl`) (`KismetMathLibrary.FClamp` (/ 50.0 (select `bool` (< _returnvalue 0.0) :`false` _returnvalue :`true` (* _returnvalue -1.0))) 2.0 100.0))
  (set `self.RotateStart` (`SceneComponent.K2_GetComponentRotation` (`self.CapsuleComponent`)))
  (bind (_direction _alpha) (`Timeline|RotateToWindowTL` :!via `PlayFromStart`)
    (:`Update`
      (`SceneComponent.K2_SetWorldRotation` (`self.CapsuleComponent`) (`KismetMathLibrary.RLerp` (`self.RotateStart`) (`SceneComponent.K2_GetComponentRotation` (`/Game/_Main/Blueprints/Interactive/BP_Window.WindowMiddlePoint` (`self.WindowREF`))) _alpha true) false false))
    (:`Finished`
      (`self.VaultOverWindow`))))

(event `VaultOverWindow`
  (bind _windowref (`self.WindowREF`))
  (bind (_returnvalue_x _returnvalue_y) (`KismetMathLibrary.BreakVector` (`SceneComponent.K2_GetComponentLocation` (`/Game/_Main/Blueprints/Interactive/BP_Window.WindowOutsidePoint` _windowref))))
  (bind (_returnvalue_x_2 _returnvalue_y_2) (`KismetMathLibrary.BreakVector` (`SceneComponent.K2_GetComponentLocation` (`/Game/_Main/Blueprints/Interactive/BP_Window.WindowInsidePoint` _windowref))))
  (`PrimitiveComponent.SetCollisionEnabled` (`self.CapsuleComponent`) "NoCollision")
  (`CharacterMovementComponent.SetMovementMode` (`self.CharacterMovement`) "MOVE_Flying" 0)
  (`|PlayMontage` (`self.Mesh`) "/Game/_Main/Blueprints/Characters/Zombie/Animation/AnimMontages/AM_VaultOverWindow.AM_VaultOverWindow" (`self.Play Rate`)
    (:`then`
      (`TimelineComponent.SetPlayRate` (`self.VaultTL`) (`self.Play Rate`))
      (bind (_direction _forward _height _rightvector) (`Timeline|VaultTL` :!via `PlayFromStart`)
        (:`Update`
          (`SceneComponent.K2_SetWorldLocation` (`self.CapsuleComponent`) (+ (* (`SceneComponent.GetRightVector` (`self.CapsuleComponent`)) _rightvector) (`KismetMathLibrary.VLerp` (`KismetMathLibrary.MakeVector` _returnvalue_x_2 _returnvalue_y_2 _height) (`KismetMathLibrary.MakeVector` _returnvalue_x _returnvalue_y _height) _forward)) false false))
        (:`Finished`
          (`self.AfterVault`))))))

(event `AfterVault`
  (if (> (`/Game/_Main/Blueprints/Components/BPC_Health.HealthCurrent` (`self.BPC_Health`)) 0.0)
    (`PrimitiveComponent.SetCollisionEnabled` (`self.CapsuleComponent`) "QueryOnly")
    (`CharacterMovementComponent.SetMovementMode` (`self.CharacterMovement`) "MOVE_Walking" 0)
    (set `self.OnLevel?` true)
    (`KismetSystemLibrary.Delay` 0.5)
    (set `/Game/_Main/Blueprints/Interactive/BP_Window.Vaulting?` false (`self.WindowREF`))
    (else
      (`CharacterMovementComponent.SetMovementMode` (`self.CharacterMovement`) "MOVE_Walking" 0)
      (set `self.OnLevel?` true)
      (set `/Game/_Main/Blueprints/Interactive/BP_Window.Vaulting?` false (`self.WindowREF`)))))

(fn `AttackRotation`
  (bind _capsulecomponent (`self.CapsuleComponent`))
  (bind (_returnvalue_roll _returnvalue_pitch _returnvalue_yaw) (`KismetMathLibrary.BreakRotator` (`KismetMathLibrary.RInterpTo` (`SceneComponent.K2_GetComponentRotation` _capsulecomponent) (`KismetMathLibrary.FindLookAtRotation` (`SceneComponent.K2_GetComponentLocation` _capsulecomponent) (`SceneComponent.K2_GetComponentLocation` (`Character.Mesh` (`GameplayStatics.GetPlayerCharacter` 0)))) (`GameplayStatics.GetWorldDeltaSeconds`) 5.0)))
  (if (`self.AttackingPlayer?`)
    (`SceneComponent.K2_SetWorldRotation` (`self.CapsuleComponent`) (`KismetMathLibrary.MakeRotator` 0.0 0.0 _returnvalue_yaw) false false)))

(fn `Calcucate Force Move TL`
  (`TimelineComponent.SetPlayRate` (`self.ForceMoveTL`) (/ 1.0 (/ (`KismetMathLibrary.Vector_Distance` (`SceneComponent.K2_GetComponentLocation` (`self.CapsuleComponent`)) (`SceneComponent.K2_GetComponentLocation` (`/Game/_Main/Blueprints/Interactive/BP_Window.WindowInsidePoint` (`self.WindowREF`)))) 200.0))))

(fn `GetEnemyREF`
  (returns (Enemy_REF :type "/Game/_Main/Blueprints/Characters/Zombie/BP_EnemyMain Object Reference"))
  (return self))

(fn `TakeDamage`
  (params (damage :type "Float (double-precision)") (BoneName :type Name) (ImpactPoint :type "Vector Structure") (Knife :type Boolean))
  (returns (`Dead?` :type Boolean) (`HeadShot?` :type Boolean))
  (locals (`Damage ` :type "Float (double-precision)") (`BoneName ` :type Name) (`ImpactPoint  ` :type "Vector Structure") (`Knife ` :type Boolean) (HeadShot :type Boolean) (RowNotFound :type Boolean) (OutRow :type "/Game/_Main/Blueprints/Structures/S_BoneHit Structure"))
  (bind _outrow_multiplier (break `/Game/_Main/Blueprints/Structures/S_BoneHit` (`local.OutRow`)))
  (bind _damage_ (`local.Damage `))
  (bind _mesh (`self.Mesh`))
  (set `local.Damage ` damage)
  (set `local.BoneName ` BoneName)
  (set `local.ImpactPoint  ` ImpactPoint)
  (set `local.HeadShot` (select `bool` Knife :`false` (select `bool` (== (`local.BoneName `) "Spine2") :`true` true)))
  (bind _returnvalue (`|GetDataTableRow` "/Game/_Main/Blueprints/DataTables/DT_BoneHit.DT_BoneHit" (`local.BoneName `))
    (:`then`
      (set `local.OutRow` _returnvalue))
    (:`RowNotFound`
      (set `local.RowNotFound` true)))
  (if Knife
    (bind _isdead_ (`/Game/_Main/Blueprints/Components/BPC_Health.HealthRemove` (`self.BPC_Health`) 200.0 0.0 false false null))
    (else
      (bind _isdead__2 (`/Game/_Main/Blueprints/Components/BPC_Health.HealthRemove` (`self.BPC_Health`) (`KismetMathLibrary.SelectFloat` (* _damage_ 0.7) (* _damage_ _outrow_multiplier) (`local.RowNotFound`)) 0.0 false false null))))
  (if (or _isdead_ _isdead__2)
    (`PrimitiveComponent.SetSimulatePhysics` _mesh true)
    (`PrimitiveComponent.SetCollisionResponseToChannel` _mesh "ECC_Visibility" "ECR_Ignore")
    (`PrimitiveComponent.SetCollisionResponseToChannel` _mesh "ECC_GameTraceChannel2" "ECR_Ignore")
    (`BlackboardComponent.SetValueAsBool` (`AIBlueprintHelperLibrary.GetBlackboard` (`AIBlueprintHelperLibrary.GetAIController` self)) "Dead" true)
    (`PrimitiveComponent.SetCollisionEnabled` (`self.CapsuleComponent`) "NoCollision")
    (`PrimitiveComponent.AddImpulse` (`self.Mesh`) (* (`local.ImpactPoint  `) -7500.0) (`local.BoneName `) false)
    (bind _asgm_co_dzombies (cast `/Game/_Main/Blueprints/Game/GM_CoDZombies` (`GameplayStatics.GetGameMode`)))
    (`/Engine/EditorBlueprintResources/StandardMacros.DecrementInt` (`/Game/_Main/Blueprints/Game/GM_CoDZombies.ZombiesAlived` _asgm_co_dzombies)
      (:`  `
        (`/Game/_Main/Blueprints/Game/GM_CoDZombies.CheckIfRoundEnd` _asgm_co_dzombies)
        (`self.DeadFade`)
        (return true (`local.HeadShot`))))
    (else
      (return false (`local.HeadShot`)))))

(fn `UserConstructionScript`
  (bind _mesh (`self.Mesh`))
  (bind _mesh_2 (`self.Mesh`))
  (bind _returnvalue (`PrimitiveComponent.CreateDynamicMaterialInstance` _mesh_2 0 (`PrimitiveComponent.GetMaterial` _mesh_2 0) "None"))
  (set `self.DynamicMaterial` _returnvalue)
  (bind _returnvalue_2 (`PrimitiveComponent.CreateDynamicMaterialInstance` _mesh 1 (`PrimitiveComponent.GetMaterial` _mesh 1) "None"))
  (set `self.DynamicMaterial1` _returnvalue_2))